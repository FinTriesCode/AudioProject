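; Oven audio Blueprint (named Ovan) that mutes ambient audio and stops a referenced TV while the player is within a check distance.
; Every Tick it compares distance to the player pawn, then re-applies and pushes a sound mix class override, silent inside the radius and default outside, where the TV restarts.
; Separate Play and Stop functions restore or zero its own audio component's volume, using the multiplier cached on BeginPlay.
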(event `self.ReceiveBeginPlay`
  (set `self.StartVol` (`AudioComponent.VolumeMultiplier` (`self.Audio`))))

(event `self.ReceiveTick`
  (params (DeltaSeconds :type "Float (single-precision)"))
  (`self.AudioCheck`))

(event `AudioCheck`
  (bind _tv_ref (`self.TV Ref`))
  (if (<= (`self.GetDistanceTo` (`GameplayStatics.GetPlayerPawn` 0)) (`self.Check Distance`))
    (`GameplayStatics.SetSoundMixClassOverride` "/Game/Audio/AmbientSoundMix.AmbientSoundMix" "/Game/Audio/SoundClasses/AmbientSoundsClass.AmbientSoundsClass" 0.0 1.0 0.0)
    (`GameplayStatics.PushSoundMixModifier` "/Game/Audio/AmbientSoundMix.AmbientSoundMix")
    (`KismetSystemLibrary.PrintText` "general audio muted")
    (`/Game/Audio/Blueprints/TvVolume_BP.TV_Stop` _tv_ref)
    (else
      (`GameplayStatics.SetSoundMixClassOverride` "/Game/Audio/AmbientSoundMix.AmbientSoundMix" "/Game/Audio/SoundClasses/AmbientSoundsClass.AmbientSoundsClass")
      (`GameplayStatics.PushSoundMixModifier` "/Game/Audio/AmbientSoundMix.AmbientSoundMix")
      (`KismetSystemLibrary.PrintText` "general audio unmuted")
      (`/Game/Audio/Blueprints/TvVolume_BP.TV_Start` _tv_ref))))

(fn `Ovan_Play`
  (`AudioComponent.SetVolumeMultiplier` (`self.Audio`) (`self.StartVol`)))

(fn `Ovan_Stop`
  (`AudioComponent.SetVolumeMultiplier` (`self.Audio`) 0.0))

(fn `UserConstructionScript`)