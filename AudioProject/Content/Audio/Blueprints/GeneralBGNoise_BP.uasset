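; GeneralBGNoise_BP is a background noise Blueprint with an Audio component and state for sound focus.
; On BeginPlay it caches the component's volume multiplier as Startvol.
; Simple getters and setters expose a focused flag and the object in focus.
; Tick is empty, and nothing in this Blueprint changes the volume or acts on the focus state.
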(event `self.ReceiveBeginPlay`
  (set `self.startvol` (`AudioComponent.VolumeMultiplier` (`self.Audio`))))

(event `self.ReceiveTick`
  (params (DeltaSeconds :type "Float (single-precision)")))

(fn `GetFocused`
  (returns (isFocused :type Boolean))
  (return (`self.soundFocused`)))

(fn `GetObjectInFocus`
  (returns (NewParam :type String))
  (return (`self.objectInFocus`)))

(fn `SetFocused`
  (params (toSet :type Boolean))
  (set `self.soundFocused` toSet))

(fn `SetObjectInFocus`
  (params (NewParam :type String))
  (set `self.objectInFocus` NewParam))

(fn `UserConstructionScript`)