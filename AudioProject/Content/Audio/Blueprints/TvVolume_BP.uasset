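; TV sound actor that gives the TV audio focus when the player pawn comes within a set distance.
; Every tick, if no sound is focused or the TV holds focus in VarCheckBP, proximity mutes ambient audio via a sound mix override and stops the Ovan sound.
; Out of range, it restores both and clears the shared flag.
; TVStart and TVStop restore or silence the TV's own volume.
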(event `self.ReceiveBeginPlay`
  (set `self.StartVol` (`AudioComponent.VolumeMultiplier` (`self.Audio`))))

(event `self.ReceiveTick`
  (params (DeltaSeconds :type "Float (single-precision)"))
  (`self.AudioCheck`))

(event `AudioCheck`
  (bind _ovan_ref (`self.Ovan Ref`))
  (if (`/Game/Audio/Blueprints/GeneralBGNoise_BP.soundFocused` (`self.VarCheckBP`))
    ;[1 1 1] Does the focus object's tring-tag match
    (bind _newparam (`/Game/Audio/Blueprints/GeneralBGNoise_BP.GetObjectInFocus` (`self.VarCheckBP`)))
    (if (`KismetStringLibrary.EqualEqual_StrStr` "TV" _newparam)
      (if (<= (`self.GetDistanceTo` (`GameplayStatics.GetPlayerPawn` 0)) (`self.Distance Check`)) :!label _label
        ;[1 1 1] Mute audio
        (`GameplayStatics.SetSoundMixClassOverride` "/Game/Audio/SoundMixes/AmbientSoundMix.AmbientSoundMix" "/Game/Audio/SoundClasses/AmbientSoundsClass.AmbientSoundsClass" 0.0 1.0 0.0)
        (`GameplayStatics.PushSoundMixModifier` "/Game/Audio/SoundMixes/AmbientSoundMix.AmbientSoundMix")
        (`KismetSystemLibrary.PrintText` "general audio muted" false)
        ;[1 1 1] Apply changes to other focused sound
        (`/Game/Audio/Blueprints/OvanAudio_BP.Ovan_Stop` _ovan_ref)
        ;[1 1 1] Update flag bool
        (set `/Game/Audio/Blueprints/GeneralBGNoise_BP.soundFocused` true (`self.VarCheckBP`))
        ;[1 1 1] Set this ot be the object in-focus
        (`/Game/Audio/Blueprints/GeneralBGNoise_BP.SetObjectInFocus` (`self.VarCheckBP`) "TV")
        (else
          ;[1 1 1] Unmute audio
          (`GameplayStatics.SetSoundMixClassOverride` "/Game/Audio/SoundMixes/AmbientSoundMix.AmbientSoundMix" "/Game/Audio/SoundClasses/AmbientSoundsClass.AmbientSoundsClass" 1.0 1.0 0.0)
          (`GameplayStatics.PushSoundMixModifier` "/Game/Audio/SoundMixes/AmbientSoundMix.AmbientSoundMix")
          (`KismetSystemLibrary.PrintText` "general audio unmuted" false)
          (`/Game/Audio/Blueprints/OvanAudio_BP.Ovan_Play` _ovan_ref)
          (set `/Game/Audio/Blueprints/GeneralBGNoise_BP.soundFocused` false (`self.VarCheckBP`)))))
    (else
      (goto _label))))

(fn `TV_Start`
  (`AudioComponent.SetVolumeMultiplier` (`self.Audio`) (`self.StartVol`)))

(fn `TV_Stop`
  (`AudioComponent.SetVolumeMultiplier` (`self.Audio`) 0.0))

(fn `UserConstructionScript`)